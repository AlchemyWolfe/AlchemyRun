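; Plains floor recipe actor that varies its look from a seed received when the reagent spawns.
; RandomizeAppearance uses seed modulo arithmetic to turn the base block in quarter steps with compensating offsets, and independently picks one of four brick placements.
; The brick slide step reads a constant zero instead of the seed, so it adds no offset.
; The branch that would hide bricks is disconnected and never runs.
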(event Custom|OnReagentSpawned
  (params (NewSeed :type Integer))
  (Variables|Default|SetSeed NewSeed)
  (CallFunction|RandomizeAppearance))

(event EventBeginPlay)

(event Collision|EventActorBeginOverlap
  (params (OtherActor :type Actor%20Object%20Reference)))

(event EventTick
  (params (DeltaSeconds :type Float%20%28single-precision%29)))

(fn ConstructionScript)

(fn RandomizeAppearance
  (bind _sm_plains_floors_block01 (Variables|Default|GetSM_Plains_Floors_Block01))
  (bind _sm_plains_floors_brick01 (Variables|Default|GetSM_Plains_Floors_Brick01))
  (bind _sm_plains_floors_brick01_2 (Variables|Default|GetSM_Plains_Floors_Brick01))
  (bind _relativelocation (Variables|/Script/Engine.SceneComponent|GetRelativeLocation _sm_plains_floors_brick01_2))
  (bind _relativelocation_2 (Variables|/Script/Engine.SceneComponent|GetRelativeLocation _sm_plains_floors_brick01))
  (bind _relativerotation (Variables|/Script/Engine.SceneComponent|GetRelativeRotation _sm_plains_floors_brick01))
  (bind _relativelocation_3 (Variables|/Script/Engine.SceneComponent|GetRelativeLocation _sm_plains_floors_block01))
  (bind _relativerotation_2 (Variables|/Script/Engine.SceneComponent|GetRelativeRotation _sm_plains_floors_block01))
  (Utilities|FlowControl|Sequence
    (:then_0
      ;[1 1 1] Rotate Base
      (switch int (Math|Integer|%(Integer) (Variables|Default|GetSeed) 4)
        (:Default
          (Transformation|SetRelativeLocationAndRotation _sm_plains_floors_block01 (Math|Vector|MakeVector (.x _relativelocation_3) (+ (.y _relativelocation_3) 5e+02) (.z _relativelocation_3)) (Math|Rotator|MakeRotator (.roll _relativerotation_2) (.pitch _relativerotation_2) (+ (.yaw _relativerotation_2) 2.7e+02)) false false))
        (:0
          (Transformation|SetRelativeLocationAndRotation _sm_plains_floors_block01 (Math|Vector|MakeVector (.x _relativelocation_3) (.y _relativelocation_3) (.z _relativelocation_3)) (Math|Rotator|MakeRotator (.roll _relativerotation_2) (.pitch _relativerotation_2) 0.0) false false))
        (:1
          (Transformation|SetRelativeLocationAndRotation _sm_plains_floors_block01 (Math|Vector|MakeVector (+ (.x _relativelocation_3) 5e+02) (.y _relativelocation_3) (.z _relativelocation_3)) (Math|Rotator|MakeRotator (.roll _relativerotation_2) (.pitch _relativerotation_2) (+ (.yaw _relativerotation_2) 9e+01)) false false))
        (:2
          (Transformation|SetRelativeLocationAndRotation _sm_plains_floors_block01 (Math|Vector|MakeVector (+ (.x _relativelocation_3) 5e+02) (+ (.y _relativelocation_3) 5e+02) (.z _relativelocation_3)) (Math|Rotator|MakeRotator (.roll _relativerotation_2) (.pitch _relativerotation_2) (+ (.yaw _relativerotation_2) 1.8e+02)) false false))))
    (:then_1
      (Utilities|FlowControl|Sequence
        (:then_0
          ;[1 1 1] Rotate Bricks
          (switch int (Math|Integer|%(Integer) (/ (Variables|Default|GetSeed) 4) 4)
            (:Default
              (Transformation|SetRelativeLocationAndRotation _sm_plains_floors_brick01 (Math|Vector|MakeVector 221.0 1.3e+02 (.z _relativelocation_2)) (Math|Rotator|MakeRotator (.roll _relativerotation) (.pitch _relativerotation) (+ (.yaw _relativerotation) 2.7e+02)) false false))
            (:0
              (Transformation|SetRelativeLocationAndRotation _sm_plains_floors_brick01 (Math|Vector|MakeVector 299.0 223.0 (.z _relativelocation_2)) (Math|Rotator|MakeRotator (.roll _relativerotation) (.pitch _relativerotation) 0.0) false false))
            (:1
              (Transformation|SetRelativeLocationAndRotation _sm_plains_floors_brick01 (Math|Vector|MakeVector 295.0 3e+02 (.z _relativelocation_2)) (Math|Rotator|MakeRotator (.roll _relativerotation) (.pitch _relativerotation) (+ (.yaw _relativerotation) 9e+01)) false false))
            (:2
              (Transformation|SetRelativeLocationAndRotation _sm_plains_floors_brick01 (Math|Vector|MakeVector 1.3e+02 296.0 (.z _relativelocation_2)) (Math|Rotator|MakeRotator (.roll _relativerotation) (.pitch _relativerotation) (+ (.yaw _relativerotation) 1.8e+02)) false false))))
        (:then_1
          ;[1 1 1] Slide Bricks
          (Transformation|SetRelativeLocation _sm_plains_floors_brick01_2 (Math|Vector|MakeVector (+ (* (Math|Conversions|ToFloat(Integer) (Math|Integer|%(Integer) 0 3)) 85.777778) (.x _relativelocation)) (+ (* (Math|Conversions|ToFloat(Integer) (Math|Integer|%(Integer) (/ 0 3) 3)) 85.777778) (.y _relativelocation)) (.z _relativelocation)) false false))))))